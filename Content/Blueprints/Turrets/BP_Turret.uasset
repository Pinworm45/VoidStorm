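; Turret Blueprint that automatically fires bullets from two arrow components on a looping timer.
; At BeginPlay it runs the parent logic, stores both arrows as sockets and starts the timer at the FireDelay interval.
; Each tick of the timer calls Fire once per socket, passing that arrow's world transform and a small, elongated bullet scale.
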(event Custom|FireAtTarget
  (for _array_element (Variables|Default|GetSockets)
    (CallFunction|Fire (Transformation|GetWorldTransform _array_element) "0.300000,0.100000,0.100000")))

(event EventBeginPlay
  (|CallParentFunction)
  (Variables|Default|SetSockets (Utilities|Array|MakeArray (Variables|Default|GetArrow) (Variables|Default|GetArrow1)))
  (Utilities|Time|SetTimerbyEvent (delegate Custom|FireAtTarget) (Variables|Default|GetFireDelay) true))

(fn ConstructionScript
  (|CallParentFunction))