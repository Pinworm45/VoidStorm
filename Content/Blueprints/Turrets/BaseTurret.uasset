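; Base turret actor that tracks an enemy ship and provides a function for firing projectiles.
; BeginPlay takes the first BaseEnemyShip found in the level as its only target and prints a debug string.
; Tick smoothly turns the whole actor toward that target with RInterpTo, without a validity check.
; Fire spawns a BaseProjectile at a supplied location, rotation and scale, but nothing in this graph calls it.
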(event EventBeginPlay
  (bind _outactors (Actor|GetAllActorsOfClass "/Game/Blueprints/EnemyShips/BaseEnemyShip.BaseEnemyShip_C"))
  (Variables|Default|SetTarget (Utilities|Array|Get(acopy) _outactors))
  (Development|PrintString "Hello"))

(event EventTick
  (params (DeltaSeconds :type Float%20%28single-precision%29))
  (Transformation|SetActorRotation (Math|Interpolation|RInterpTo (Transformation|GetActorRotation) (Math|Rotator|FindLookatRotation (Transformation|GetActorLocation) (Transformation|GetActorLocation (Variables|Default|GetTarget))) DeltaSeconds 1.0)))

(fn ConstructionScript)

(fn Fire
  (params (BulletLocation&Rotation :type Transform) (BulletScale :type Vector))
  (bind (_location _rotation) (Math|Transform|BreakTransform BulletLocation&Rotation))
  (Game|SpawnActorfromClass "/Game/Blueprints/Weapons/BaseProjectile.BaseProjectile_C" (Math|Transform|MakeTransform _location _rotation BulletScale) "AlwaysSpawn" 0 0))